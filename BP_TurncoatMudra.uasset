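; BP_TurncoatMudra is a spell action that temporarily turns an enemy AI to fight for the caster's team.
; At its notable point it takes the lock-on target, falling back to a camera-yaw capsule trace.
; TurnEnemy stops the target's action, swaps its team and aims it at the closest non-allied AI found by sphere trace, with an attached effect.
; After the duration it restores the team and retargets the caster; invalid targets refund Focus.
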(event EventOnNotablePointReached
  (bind _characterowner (Variables|Default|GetCharacterOwner))
  (bind _characterowner_2 (Variables|Default|GetCharacterOwner))
  (bind _characterowner_3 (Variables|Default|GetCharacterOwner))
  (bind _returnvalue (Pawn|GetController _characterowner_3))
  (bind _returnvalue_2 (Transformation|GetActorLocation _characterowner))
  (bind _returnvalue_3 (Actor|GetComponentbyClass _characterowner_2 "/Script/Engine.CameraComponent"))
  (bind _returnvalue_4 (Transformation|GetWorldLocation _returnvalue_3))
  (bind _returnvalue_5 (Transformation|GetWorldRotation _returnvalue_3))
  (bind _returnvalue_6 (Actor|GetComponentbyClass _returnvalue "/Script/TargetingSystem.ATSTargetingComponent"))
  (bind _returnvalue_7 (Transformation|GetWorldLocation _returnvalue_3))
  (bind _yaw (Math|Rotator|BreakRotator _returnvalue_5))
  (bind _returnvalue_8 (Class|ATSBaseTargetComponent|GetCurrentTarget _returnvalue_6))
  (bind _returnvalue_9 (Math|Rotator|MakeRotator 0.0 0.0 _yaw))
  (bind _returnvalue_10 (Math|Vector|GetForwardVector _returnvalue_9))
  (bind _returnvalue_11 (* _returnvalue_10 1.5e+03))
  (bind _returnvalue_12 (+ _returnvalue_4 _returnvalue_11))
  ;[1 1 1] Setting spell target if locked on, checking it's valid and getting it's AI controller
  (|CallParentFunction)
  (Class|ACFBaseAction|PlayEffects)
  (bind _output_get (Variables|Default|SetspellTarget _returnvalue_8))
  (Utilities|IsValid _output_get
    (:Is%20Valid
      (Utilities|TurnEnemy (Actor|GetComponentbyClass _returnvalue_8 "/Script/ActionsSystem.ACFActionsManagerComponent") (AI|GetAIController _returnvalue_8)))
    (:Is%20Not%20Valid
      ;[1 1 1] Setting spell target if not locked on using capsule trace, checking it's valid and getting it's AI controller
      (bind _outhit (Class|KismetSystemLibrary|CapsuleTraceSingleforObjects (Math|Vector|MakeVector (.x _returnvalue_7) (.y _returnvalue_7) (.z _returnvalue_2)) (Math|Vector|MakeVector (.x _returnvalue_12) (.y _returnvalue_12) (.z _returnvalue_2)) 2e+02 1e+02 (Utilities|Array|MakeArray "ObjectTypeQuery3") false 0 "None" true))
      (bind _output_get_2 (Variables|Default|SetspellTarget (.HitActor (Collision|BreakHitResult _outhit))))
      (Utilities|TurnEnemy (Actor|GetComponentbyClass _output_get_2 "/Script/ActionsSystem.ACFActionsManagerComponent") (AI|GetAIController (.HitActor (Collision|BreakHitResult _outhit)))))))

(fn PlaySpellEffect
  (params (Target :type Actor%20Object%20Reference))
  (bind _returnvalue (Niagara|SpawnSystemAttached (Variables|Default|GetspellEffect) (Actor|GetComponentbyClass Target "/Script/Engine.SkeletalMeshComponent") "None" "0, 0, 0" "0, 0, 0" "KeepRelativeOffset" false))
  (return _returnvalue))

(fn FindTarget
  (params (SpherePos :type Vector))
  ;[1 1 1] Getting all targets near the turned enemy and storing them in an array
  (bind _outhits (Collision|MultiSphereTraceForObjects (Transformation|GetActorLocation (Variables|Default|GetspellTarget)) "0, 0, 0" 6e+04 (Utilities|Array|MakeArray "ObjectTypeQuery3") false 0 "None"))
  (for _array_element _outhits
    (Variables|Default|SetnewEnemyTarget (.hitactor _array_element))
    (bind _asacfaicontroller (Utilities|Casting|CastToACFAIController (AI|GetAIController (.hitactor _array_element))))
    ;[1 1 1] Check if target is not on the player's team
    (if (not (Utilities|Enum|Equal(Enum) (Variables|Default|GetcasterTeam) (Variables|/Script/AIFramework.ACFBaseAIController|GetCombatTeam _asacfaicontroller)))
      ;[1 1 1] Check if target distance is closer then the current closet target distance
      (bind _output_get (Variables|Default|SettargetDistance (Math|Vector|Distance(Vector) (Transformation|GetActorLocation (Variables|Default|GetspellTarget)) (Transformation|GetActorLocation (Variables|Default|GetnewEnemyTarget)))))
      (if (< _output_get (Variables|Default|GetclosestTargetDistance))
        ;[1 1 1] Closet Target distance is set to target distance and the closet enemy target is replaced with the new enemy target
        (Variables|Default|SetclosestTargetDistance (Variables|Default|GettargetDistance))
        (Variables|Default|SetclosetEnemyTarget (Variables|Default|GetnewEnemyTarget)))))
  (return (Variables|Default|GetclosetEnemyTarget)))